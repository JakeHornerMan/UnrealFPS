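; BP_Zombie is a zombie character that takes damage, tracks health through a BPCHealth component and can ragdoll.
; BeginPlay binds the component's death and hit dispatchers, while AnyDamage lowers health and calls Died or Hit, which only print messages.
; DamageResponse accumulates damage and reports neck-bone criticals and death, with its ragdoll branch left unconnected.
; Server events apply damage and relay a multicast ragdoll that enables mesh physics, disables capsule collision and adds an impulse.
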(event `self.ReceiveBeginPlay`
  (bind _bpc_health (`self.BPC_Health`))
  (`|ExecutionSequence`
    (:`then_0`
      ;[0.3851 1 0.3241] Event displatcher for health events
      (add `/Game/Blueprints/Bios/BPC_Health.DeathEventDispatcher` _bpc_health (`|CreateDelegate` :!event `Died`))
      (add `/Game/Blueprints/Bios/BPC_Health.HitEventDispatcher` _bpc_health (`|CreateDelegate` :!event `Hit`)))))

(event `ApplyDamageSERVER`
  (params (DamagedActor :type "Actor Object Reference") (BaseDamage :type "Float (single-precision)") (DamageCauser :type "Actor Object Reference"))
  ;[0 1 0.8157] Apply Damage MULTIPLAYER
  (`GameplayStatics.ApplyDamage` DamagedActor BaseDamage null DamageCauser))

(event `self.ReceiveAnyDamage`
  (params (Damage :type "Float (single-precision)") (DamageType :type "DamageType Object Reference") (InstigatedBy :type "Controller Object Reference") (DamageCauser :type "Actor Object Reference"))
  (bind _bpc_health (`self.BPC_Health`))
  ;[0.3367 1 0.2681] Apply Damage
  (bind _output_get (set `/Game/Blueprints/Bios/BPC_Health.Health` (- (`/Game/Blueprints/Bios/BPC_Health.Health` _bpc_health) Damage) _bpc_health))
  (if (`self.DebugLog`)
    (`KismetSystemLibrary.PrintString` (`KismetStringLibrary.BuildString_Double` "Zombie, " "Health: " _output_get) true true (struct :`R` 1.0 :`G` 0.645766 :`A` 1.0)))
  (if (<= (`/Game/Blueprints/Bios/BPC_Health.Health` (`self.BPC_Health`)) 0.0)
    (`self.Died`)
    (else
      (`self.Hit`))))

(event `RagdollSERVER`
  (`self.RagdollMULTICAST`))

(event `RagdollMULTICAST`
  (`self.RagDoll` "neck_01" (100.0 100.0 100.0)))

(fn `DamageResponse`
  (params (Amount :type "Float (double-precision)") (BoneName :type Name) (ImpactPoint :type "Vector Structure") (Knife :type Boolean) (DamagedActor :type "Actor Object Reference"))
  (returns (IsCriticalHit :type Boolean) (IsDead :type Boolean))
  (locals (Crit :type Boolean) (Dead :type Boolean) (BoneHit :type Name) (ImpactPointHit :type "Vector Structure"))
  (set `local.ImpactPointHit` ImpactPoint)
  (bind _output_get (set `local.BoneHit` BoneName))
  (set `local.Crit` (== _output_get "neck_01"))
  (bind _output_get_2 (set `self.DamageTaken` (+ Amount (`self.DamageTaken`))))
  (bind _output_get_3 (set `local.Dead` (>= _output_get_2 (`/Game/Blueprints/Bios/BPC_Health.Health` (`self.BPC_Health`)))))
  (return (`local.Crit`) (`local.Dead`)))

(fn `Died`
  (`KismetSystemLibrary.PrintString` "Zombie has died"))

(fn `Hit`
  (`KismetSystemLibrary.PrintString` "Zombie has been hit"))

(fn `RagDoll`
  (params (BoneName :type Name) (A :type "Vector Structure") (Target :type "PrimitiveComponent Object Reference"))
  (bind _mesh (`self.Mesh`))
  (`PrimitiveComponent.SetSimulatePhysics` _mesh true)
  (`PrimitiveComponent.SetSimulatePhysics` Target true)
  (`PrimitiveComponent.SetCollisionResponseToChannel` _mesh "ECC_Visibility" "ECR_Ignore")
  (`PrimitiveComponent.SetCollisionEnabled` (`self.CapsuleComponent`) "NoCollision")
  (`PrimitiveComponent.AddImpulse` (`self.Mesh`) (* A -20000.0) BoneName false))

(fn `UserConstructionScript`)