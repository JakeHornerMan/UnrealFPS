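; Base weapon Blueprint that swaps its skeletal mesh and keeps per-gun hip and aim offsets.
; The changeWeapon event sets the new mesh, then SetAimOffForWeapon prints the asset's display name and switches on it.
; Matching rifle names pass hard-coded location and rotation values to SetDeafultGunLocations, which stores them in the aim and hip offset variables.
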(event `self.ReceiveBeginPlay`)

(event `changeWeapon`
  (params (NewMesh :type "SkeletalMesh Object Reference"))
  (`SkeletalMeshComponent.SetSkeletalMeshAsset` (`self.SkeletalMesh`) NewMesh)
  (`self.SetAimOffForWeapon`))

(fn `SetAimOffForWeapon`
  (bind _returnvalue (`KismetSystemLibrary.GetDisplayName` (`SkinnedMeshComponent.GetSkinnedAsset` (`self.SkeletalMesh`))))
  (`KismetSystemLibrary.PrintString` _returnvalue)
  (switch `string` _returnvalue
    (:`assault_rifle_a`
      (`self.SetDeafultGunLocations` (15.0 15.6 4.4) (struct :`Pitch` 16.339324 :`Yaw` 89.69528 :`Roll` -8.512689) (0.0 4.0 3.0) (struct :`Pitch` 10.0 :`Yaw` 98.0 :`Roll` 1.8)))
    (:`ak47`
      (`self.SetDeafultGunLocations` (3.673152 13.540247 12.658118) (struct :`Pitch` 14.980173 :`Yaw` 90.206525 :`Roll` -13.209565) (-20.0 3.4 15.2) (struct :`Pitch` 15.0 :`Yaw` 90.0 :`Roll` -5.0)))))

(fn `SetDeafultGunLocations`
  (params (AimLocation :type "Vector Structure") (AimRotation :type "Rotator Structure") (HipLocation :type "Vector Structure") (HipRotation :type "Rotator Structure"))
  (set `self.AimOffsetLoc` AimLocation)
  (set `self.AimOffsetRot` AimRotation)
  (set `self.HipOffsetLoc` HipLocation)
  (set `self.HipOffsetRot` HipRotation))

(fn `UserConstructionScript`)