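; Inventory component that tracks weapon ammo in an array of entries, each holding an item ID, magazine ammo and total ammo.
; RemoveAmmoMag and ReloadGun events wrap functions that decrement a magazine or set it to a given amount, with optional debug printing.
; Reload returns leftover rounds to the total before deducting the new magazine, without clamping to available ammo.
; Helper functions report whether a magazine is empty or full.
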(event `RemoveAmmoMag`
  (params (Index :type Integer) (Debug :type Boolean))
  (`self.Remove Ammo Magazine` Index Debug))

(event `ReloadGun`
  (params (Index :type Integer) (`MagazineAmount ` :type Integer) (Debug :type Boolean))
  (`self.Reload` Index `MagazineAmount ` Debug))

(fn `IsMagazineEmpty`
  (params (Index :type Integer))
  (returns (IsEmpty :type Boolean))
  (bind (_output_id _output_magazineammo) (break `/Game/Blueprints/Inventory/DynamicInventoryItem` (`|GetArrayItem` (`self.Inventory`) Index)))
  (return (<= _output_magazineammo 0)))

(fn `IsMagazineFull`
  (params (Index :type Integer) (FullMagAmmount :type Integer))
  (returns (IsFull :type Boolean))
  (bind (_output_id _output_magazineammo) (break `/Game/Blueprints/Inventory/DynamicInventoryItem` (`|GetArrayItem` (`self.Inventory`) Index)))
  (return (>= _output_magazineammo FullMagAmmount)))

(fn `Reload`
  (params (Index :type Integer) (MagazineAmmo :type Integer) (Debug :type Boolean))
  (bind _inventory (`self.Inventory`))
  (bind (_output_id _output_magazineammo _output_totalammo) (break `/Game/Blueprints/Inventory/DynamicInventoryItem` (`|GetArrayItem` _inventory Index)))
  (bind (_output_id_2 _output_magazineammo_2 _output_totalammo_2) (break `/Game/Blueprints/Inventory/DynamicInventoryItem` (`|GetArrayItem` (`self.Inventory`) Index)))
  (`KismetArrayLibrary.Array_Set` _inventory Index (make `/Game/Blueprints/Inventory/DynamicInventoryItem` _output_id MagazineAmmo (+ _output_magazineammo (- _output_totalammo MagazineAmmo))))
  (if Debug
    (`KismetSystemLibrary.PrintString` (`KismetStringLibrary.BuildString_Int` (`KismetStringLibrary.BuildString_Int` (`KismetStringLibrary.BuildString_Int` "" "Current Weapon: " _output_id_2) ", Mag Ammo:" _output_magazineammo_2) ", Total Ammo:" _output_totalammo_2))))

(fn `Remove Ammo Magazine`
  (params (Index :type Integer) (Debug :type Boolean))
  (locals (WeaponIndex :type Integer))
  (bind _inventory (`self.Inventory`))
  (bind (_output_id _output_magazineammo) (break `/Game/Blueprints/Inventory/DynamicInventoryItem` (`|GetArrayItem` (`self.Inventory`) (`local.WeaponIndex`))))
  (bind _output_get (set `local.WeaponIndex` Index))
  (bind (_output_id_2 _output_magazineammo_2 _output_totalammo) (break `/Game/Blueprints/Inventory/DynamicInventoryItem` (`|GetArrayItem` _inventory _output_get)))
  (`KismetArrayLibrary.Array_Set` _inventory _output_get (make `/Game/Blueprints/Inventory/DynamicInventoryItem` _output_id_2 (- _output_magazineammo_2 1) _output_totalammo))
  (if Debug
    (`KismetSystemLibrary.PrintString` (`KismetStringLibrary.Conv_IntToString` _output_magazineammo) true true (struct :`R` 1.0 :`G` 0.835543 :`A` 1.0))))